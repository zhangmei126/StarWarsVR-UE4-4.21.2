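; Blaster-style laser bolt projectile that can be deflected by lightsabers, with size, speed and color set in the construction script.
; Blocking hits notify the struck actor, spawn velocity-driven sparks, play an impact or ricochet sound and destroy the bolt.
; Overlapping another bolt destroys it, while saber overlaps redirect it along the saber's deflect vector, speeding it up with swing force.
; A separate Hit event applies damage and destroys thermal detonators.
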(event OnComponentBeginOverlap(Box)
  (params (OverlappedComponent :type Primitive%20Component%20Object%20Reference) (OtherActor :type Actor%20Object%20Reference) (OtherComp :type Primitive%20Component%20Object%20Reference) (OtherBodyIndex :type Integer) (bFromSweep :type Boolean) (SweepResult :type Hit%20Result%20Structure%20%28by%20ref%29))
  (bind _projectilemovement (Variables|Default|GetProjectileMovement))
  ;[1 1 1] Laser Overlap (Mostly for saber collision)
  (bind _returnvalue (Effects|SpawnEmitteratLocation "/Game/Lightsaber/Effects/P_Sparks.P_Sparks" (Math|Vector|SelectVector (.Location (Collision|BreakHitResult SweepResult)) (Transformation|GetWorldLocation (Variables|Default|GetStaticMesh)) bFromSweep)))
  (Utilities|FlowControl|Sequence
    (:then_0
      (Utilities|Casting|CastToBP_LaserBullet OtherActor)
      (Effects|Components|ParticleSystem|SetVectorParameter _returnvalue "Force" (/ (Variables|/Script/Engine.MovementComponent|GetVelocity (Variables|Default|GetProjectileMovement)) 2.0))
      (Utilities|FlowControl|Sequence
        (:then_0
          (bind _item (Utilities|RandomItem (Variables|Default|GetSaberHitSounds) :!label _label)
            (:Get
              (Audio|PlaySoundatLocation _item (Transformation|GetWorldLocation (Variables|Default|GetStaticMesh)) "0, 0, 0" 1.0 1.0 0.0 "/Game/Lightsaber/Sound/SaberSounds/SA_Basic.SA_Basic" 0 0))))
        (:then_1
          (Actor|DestroyActor))))
    (:then_1
      (bind _asbp_saber_base (Utilities|Casting|CastToBP_SaberBase OtherActor))
      (Effects|Components|ParticleSystem|SetVectorParameter _returnvalue "Force" (+ (* (Variables|/Game/Lightsaber/Blueprints/BP_SaberBase.BP_SaberBase_C|GetlastForce _asbp_saber_base) 4e+01) (* (Default|GetDeflect _asbp_saber_base) 3e+02)))
      (Variables|/Script/Engine.MovementComponent|SetVelocity _projectilemovement (* (* (Default|GetDeflect _asbp_saber_base) (Math|Vector|VectorLength (Variables|/Script/Engine.MovementComponent|GetVelocity _projectilemovement))) (Math|Float|Clamp(Float) (/ (Math|Vector|VectorLength (Variables|/Game/Lightsaber/Blueprints/BP_SaberBase.BP_SaberBase_C|GetlastForce _asbp_saber_base)) 15.0) 1.0 3.0)))
      (goto _label))))

(event OnComponentHit(Box)
  (params (HitComponent :type Primitive%20Component%20Object%20Reference) (OtherActor :type Actor%20Object%20Reference) (OtherComp :type Primitive%20Component%20Object%20Reference) (NormalImpulse :type Vector :default "0, 0, 0") (Hit :type Hit%20Result%20Structure%20%28by%20ref%29))
  (bind (_bblockinghit _binitialoverlap _time _distance _location _impactpoint _normal _impactnormal _physmat _hitactor _hitcomponent) (Collision|BreakHitResult Hit))
  (bind _projectilemovement (Variables|Default|GetProjectileMovement))
  (bind _velocity (Variables|/Script/Engine.MovementComponent|GetVelocity _projectilemovement))
  ;[1 1 1] Hit
  (Class|BIShot|GetShot(Message) OtherActor _velocity Hit)
  (bind _returnvalue (Effects|SpawnEmitteratLocation "/Game/Lightsaber/Effects/P_Sparks.P_Sparks" (+ _impactpoint (* _impactnormal 5.0))))
  (Effects|Components|ParticleSystem|SetVectorParameter _returnvalue "Force" (/ _velocity 8.0))
  (Utilities|FlowControl|Sequence
    (:then_0
      (if (Variables|Default|GetCanPlaySound)
        (if (>= (Math|Random|RandomFloatinRange 0.0 1.0) 0.2)
          (Audio|PlaySoundatLocation "/Game/Lightsaber/Sound/BlasterSounds/Impacts/impact2_Cue.impact2_Cue" _impactpoint "0, 0, 0" 1.0 1.0 0.0 0 0 0)
          (else
            (Audio|PlaySoundatLocation "/Game/Lightsaber/Sound/BlasterSounds/Impacts/ricochet_Cue.ricochet_Cue" _impactpoint "0, 0, 0" 1.0 1.0 0.0 0 0 0)))))
    (:then_1
      (Actor|DestroyActor))))

(event Collision|EventHit
  (params (MyComp :type Primitive%20Component%20Object%20Reference) (Other :type Actor%20Object%20Reference) (OtherComp :type Primitive%20Component%20Object%20Reference) (bSelfMoved :type Boolean) (HitLocation :type Vector :default "0, 0, 0") (HitNormal :type Vector :default "0, 0, 0") (NormalImpulse :type Vector :default "0, 0, 0") (Hit :type Hit%20Result%20Structure%20%28by%20ref%29))
  (CallFunction|CasttoActors&DoDamage false Other)
  (bind _asbp_thermal_detonator (Utilities|Casting|CastToBP_ThermalDetonator Other))
  (Default|Destroy _asbp_thermal_detonator))

(fn ConstructionScript
  (bind _collisionmult (Variables|Default|GetCollisionMult))
  (bind _width (Variables|Default|GetWidth))
  (bind _width_2 (Variables|Default|GetWidth))
  (bind _color (Variables|Default|GetColor))
  (bind _returnvalue (* _width_2 _collisionmult))
  (Transformation|SetWorldScale3D (Variables|Default|GetStaticMesh) (Math|Vector|MakeVector (Variables|Default|GetLength) _width _width))
  (Components|Box|SetBoxExtent (Variables|Default|GetBox) (Math|Vector|MakeVector (* (Variables|Default|GetLength) 8.0 (Variables|Default|GetCollisionMult)) _returnvalue _returnvalue) true)
  (Variables|/Script/Engine.MovementComponent|SetVelocity (Variables|Default|GetProjectileMovement) (Math|Vector|MakeVector (Variables|Default|GetVelocity) 0.0 0.0))
  (bind _returnvalue_2 (Rendering|Material|CreateDynamicMaterialInstance (Variables|Default|GetStaticMesh) 0 "/Game/Lightsaber/Materials/Lightsaber/M_Saber_Base.M_Saber_Base" "None" :!class /Script/Engine.PrimitiveComponent))
  (Rendering|Material|SetVectorParameterValue _returnvalue_2 "Color" _color :!class /Script/Engine.MaterialInstanceDynamic)
  (Rendering|Components|Light|SetLightColor (Variables|Default|GetPointLight) _color true))