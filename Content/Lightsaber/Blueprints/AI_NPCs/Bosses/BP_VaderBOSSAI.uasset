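; Darth Vader boss AI for the lightsaber game, turning on its child-actor saber at start and moving toward any motion-controller pawn it sees.
; A combat flag, set on sight or for three seconds after non-lethal hits, drives walk speed and breathing sound on Tick.
; Damage picks random saber or regular hit markers through a shared helper.
; Death plays a random animation with explosion and smoke, then destroys the actor.
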(event OnSeePawn(PawnSensing)
  (params (Pawn :type Pawn%20Object%20Reference))
  (Variables|Default|SetInCombat? true)
  (bind _asbp_motion_controller_pawn (Utilities|Casting|CastToBP_MotionControllerPawn Pawn))
  (AI|AIMoveTo self "0, 0, 0" _asbp_motion_controller_pawn 5.0 false
    (:OnSuccess
      _)
    (:OnFail
      _))
  (Variables|Default|SetInCombat? false))

(event Custom|DeathSequence
  (bind _sphere (Variables|Default|GetSphere))
  (bind _returnvalue (Transformation|GetWorldLocation _sphere))
  (Development|PrintString "BerserkerDEAD")
  (Effects|SpawnEmitteratLocation "/Game/StarterContent/Particles/P_Explosion.P_Explosion" _returnvalue)
  (bind _item (Utilities|RandomItem (Variables|Default|GetDeathAnims))
    (:Get
      (Components|Animation|PlayAnimation (Variables|Character|GetMesh) _item false)
      (Variables|Default|SetCanTakeDamage false)
      (Components|DestroyComponent (Variables|Collision|GetCapsuleComponent))
      (Utilities|FlowControl|Delay 3.0)
      (Effects|SpawnEmitteratLocation "/Game/StarterContent/Particles/SmokeBurst.SmokeBurst" _returnvalue)
      (Actor|DestroyActor))))

(event Custom|Panic
  (Variables|Default|SetInCombat? true)
  (Utilities|FlowControl|Delay 3.0)
  (Variables|Default|SetInCombat? false))

(event EventBeginPlay
  (bind _asvader_saber_1 (Utilities|Casting|CastToVaderSaber1 (Variables|/Script/Engine.ChildActorComponent|GetChildActor (Variables|Default|GetSaber))))
  (Default|Turnon _asvader_saber_1))

(event EventTick
  (params (DeltaSeconds :type Float%20%28single-precision%29))
  (bind _breathing (Variables|Default|GetBreathing))
  (bind _charactermovement (Variables|Character|GetCharacterMovement))
  (if (Variables|Default|GetInCombat?)
    (Variables|/Script/Engine.CharacterMovementComponent|SetMaxWalkSpeed _charactermovement 3.5e+02)
    (Audio|Components|Audio|SetSound _breathing "/Game/BF2_Assets/Characters/Vader/sounds/SW01_Characters_Heroes_DarthVader_Breathing_Normal_VAR_01_Cue.SW01_Characters_Heroes_DarthVader_Breathing_Normal_VAR_01_Cue")
    (else
      (Variables|/Script/Engine.CharacterMovementComponent|SetMaxWalkSpeed _charactermovement 2e+02)
      (Audio|Components|Audio|SetSound _breathing "/Game/BF2_Assets/Characters/Vader/sounds/SW01_Characters_Heroes_DarthVader_Breathing_Slow_VAR_01_Cue.SW01_Characters_Heroes_DarthVader_Breathing_Slow_VAR_01_Cue"))))

(fn ConstructionScript)

(fn TakeDamage
  (bind _issaber_ (Variables|Default|GetIsSaber?))
  (if _issaber_
    (bind _item (Utilities|RandomItem (Variables|Default|GetSaberHitMarkers))
      (:Get
        _))
    (else
      (bind _item_2 (Utilities|RandomItem (Variables|Default|GetHitMarkers))
        (:Get
          _))))
  (bind (_isdead _newhealth) (CallFunction|TakeDamage (Variables|Default|GetCanTakeDamage) (Variables|Default|GetHealth) (select _issaber_ _item _item_2) (Variables|Default|GetIsSaber?)))
  (Variables|Default|SetHealth _newhealth)
  (if _isdead
    (CallFunction|DeathSequence)
    (else
      (CallFunction|Panic))))

(fn GetTarget
  (return (Transformation|GetWorldLocation (Variables|Default|GetSphere))))