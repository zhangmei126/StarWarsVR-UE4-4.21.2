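; BX enemy NPC character that takes saber or other hits and speeds up when in combat.
; TakeDamage picks a random hit marker by damage type and updates health through a TakeDamage helper, triggering either death or a brief Panic combat state.
; Tick switches walk speed on that state, and GetTarget exposes the Sphere's location as a target point.
; Death plays an explosion and random animation, removes the capsule, then destroys the actor in a smoke burst.
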(event Custom|DeathSequence
  (bind _sphere (Variables|Default|GetSphere))
  (bind _returnvalue (Transformation|GetWorldLocation _sphere))
  (Development|PrintString "BX DEAD")
  (Effects|SpawnEmitteratLocation "/Game/StarterContent/Particles/P_Explosion.P_Explosion" _returnvalue "0, 0, 0" "0.800000,0.800000,0.800000")
  (bind _item (Utilities|RandomItem (Variables|Default|GetDeathAnims))
    (:Get
      (Components|Animation|PlayAnimation (Variables|Character|GetMesh) _item false)
      (Variables|Default|SetCanTakeDamage false)
      (Components|DestroyComponent (Variables|Collision|GetCapsuleComponent))
      (Utilities|FlowControl|Delay 3.0)
      (Effects|SpawnEmitteratLocation "/Game/StarterContent/Particles/SmokeBurst.SmokeBurst" _returnvalue)
      (Actor|DestroyActor))))

(event Custom|Panic
  (Variables|Default|SetInCombat? true)
  (Utilities|FlowControl|Delay 3.0)
  (Variables|Default|SetInCombat? false))

(event EventBeginPlay)

(event Collision|EventActorBeginOverlap
  (params (OtherActor :type Actor%20Object%20Reference)))

(event EventTick
  (params (DeltaSeconds :type Float%20%28single-precision%29))
  (bind _charactermovement (Variables|Character|GetCharacterMovement))
  (if (Variables|Default|GetInCombat?)
    (Variables|/Script/Engine.CharacterMovementComponent|SetMaxWalkSpeed _charactermovement 5e+02)
    (else
      (Variables|/Script/Engine.CharacterMovementComponent|SetMaxWalkSpeed _charactermovement 1.5e+02))))

(fn ConstructionScript)

(fn TakeDamage
  (bind _issaber_ (Variables|Default|GetIsSaber?))
  (if _issaber_
    (bind _item (Utilities|RandomItem (Variables|Default|GetSaberHitMarkers))
      (:Get
        _))
    (else
      (bind _item_2 (Utilities|RandomItem (Variables|Default|GetHitMarkers))
        (:Get
          _))))
  (bind (_isdead _newhealth) (CallFunction|TakeDamage (Variables|Default|GetCanTakeDamage) (Variables|Default|GetHealth) (select _issaber_ _item _item_2) (Variables|Default|GetIsSaber?)))
  (Variables|Default|SetHealth _newhealth)
  (if _isdead
    (CallFunction|DeathSequence)
    (else
      (CallFunction|Panic))))

(fn GetTarget
  (return (Transformation|GetWorldLocation (Variables|Default|GetSphere))))