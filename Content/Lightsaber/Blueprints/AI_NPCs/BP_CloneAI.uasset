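; Clone AI character that chases the VR motion-controller pawn on sight and can be killed by saber or other hits.
; Sighting, damage panic or Sprint sets InCombat, which Tick uses to switch between walk and run speeds.
; TakeDamage picks a random saber or regular hit marker, updates health, then triggers Panic or death.
; Death plays a random animation and smoke, then drops a random DC17 or DC15 before destroying the actor.
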(event OnSeePawn(PawnSensing)
  (params (Pawn :type Pawn%20Object%20Reference))
  (Variables|Default|SetInCombat? true)
  (bind _asbp_motion_controller_pawn (Utilities|Casting|CastToBP_MotionControllerPawn Pawn))
  (AI|AIMoveTo self "0, 0, 0" _asbp_motion_controller_pawn 5.0 false
    (:OnSuccess
      _)
    (:OnFail
      _))
  (Variables|Default|SetInCombat? false))

(event Custom|DeathSequence
  (bind _sphere (Variables|Default|GetSphere))
  (bind _returnvalue (Transformation|GetWorldLocation _sphere))
  (Development|PrintString "Clone DEAD")
  (Effects|SpawnEmitteratLocation "/Game/StarterContent/Particles/SmokeBurst.SmokeBurst" _returnvalue)
  (bind _item (Utilities|RandomItem (Variables|Default|GetDeathAnims))
    (:Get
      (Components|Animation|PlayAnimation (Variables|Character|GetMesh) _item false)
      (Variables|Default|SetCanTakeDamage false)
      (Components|DestroyComponent (Variables|Collision|GetCapsuleComponent))
      (Utilities|FlowControl|Delay 3.0)
      (Effects|SpawnEmitteratLocation "/Game/StarterContent/Particles/SmokeBurst.SmokeBurst" _returnvalue)
      (Game|SpawnActorfromClass (select (>= (Math|Random|RandomFloatinRange 0.0 1.0) 0.5) "/Game/Lightsaber/Blueprints/BlasterBPs/DC17.DC17_C" "/Game/Lightsaber/Blueprints/BlasterBPs/DC15.DC15_C") (Math|Transform|MakeTransform _returnvalue "0, 0, 0" "1,1,1") "Undefined" 0 0)
      (Actor|DestroyActor))))

(event Custom|Panic
  (Variables|Default|SetInCombat? true)
  (Utilities|FlowControl|Delay 3.0)
  (Variables|Default|SetInCombat? false))

(event EventBeginPlay)

(event Collision|EventActorBeginOverlap
  (params (OtherActor :type Actor%20Object%20Reference)))

(event EventTick
  (params (DeltaSeconds :type Float%20%28single-precision%29))
  (bind _charactermovement (Variables|Character|GetCharacterMovement))
  (if (Variables|Default|GetSprint?)
    (Variables|Default|SetInCombat? true))
  (if (Variables|Default|GetInCombat?)
    (Variables|/Script/Engine.CharacterMovementComponent|SetMaxWalkSpeed _charactermovement 425.0)
    (else
      (Variables|/Script/Engine.CharacterMovementComponent|SetMaxWalkSpeed _charactermovement 1.5e+02))))

(fn ConstructionScript)

(fn TakeDamage
  (bind _issaber_ (Variables|Default|GetIsSaber?))
  (if _issaber_
    (bind _item (Utilities|RandomItem (Variables|Default|GetSaberHitMarkers))
      (:Get
        _))
    (else
      (bind _item_2 (Utilities|RandomItem (Variables|Default|GetHitMarkers))
        (:Get
          _))))
  (bind (_isdead _newhealth) (CallFunction|TakeDamage (Variables|Default|GetCanTakeDamage) (Variables|Default|GetHealth) (select _issaber_ _item _item_2) (Variables|Default|GetIsSaber?)))
  (Variables|Default|SetHealth _newhealth)
  (if _isdead
    (CallFunction|DeathSequence)
    (else
      (CallFunction|Panic))))

(fn GetTarget
  (return (Transformation|GetWorldLocation (Variables|Default|GetSphere))))