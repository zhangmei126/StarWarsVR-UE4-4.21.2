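; Dual-bladed lightsaber handle Blueprint that extends a parent handle with a second blade, Saber2.
; Crystal use, turn-on and turn-off call the parent logic, then mirror color or power onto the second blade.
; A face button toggles only the second blade, and it ignites only when a crystal is present or none is required.
; The construction script applies the base color to the second blade.
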(event EventBeginPlay)

(event Collision|EventActorBeginOverlap
  (params (OtherActor :type Actor%20Object%20Reference)))

(event EventUseCrystal
  (params (Crystal :type BP%20Crystal%20Object%20Reference))
  (|CallParentFunction Crystal)
  (Default|SetColor (CallFunction|GetChildSaber (Variables|Default|GetSaber2)) (Variables|/Game/Lightsaber/Blueprints/MiscObjects/BP_Crystal.BP_Crystal_C|Getcolor Crystal)))

(event EventTick
  (params (DeltaSeconds :type Float%20%28single-precision%29)))

(event EventFaceButton2Press
  (if (or (Variables|Default|GethasCrystal) (not (Variables|Default|GetrequireCrystal)))
    (Default|TurnToggle (CallFunction|GetChildSaber (Variables|Default|GetSaber2)))))

(event EventTurnOff
  (|CallParentFunction)
  (Default|TurnOff (CallFunction|GetChildSaber (Variables|Default|GetSaber2))))

(event EventTurnon
  (|CallParentFunction)
  (if (or (Variables|Default|GethasCrystal) (not (Variables|Default|GetrequireCrystal)))
    (Default|Turnon (CallFunction|GetChildSaber (Variables|Default|GetSaber2)))))

(fn ConstructionScript
  (|CallParentFunction)
  (Default|SetColor (CallFunction|GetChildSaber (Variables|Default|GetSaber2)) (Variables|Default|GetbaseColor)))