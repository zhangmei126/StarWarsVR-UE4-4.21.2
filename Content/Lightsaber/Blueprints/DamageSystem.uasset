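; DamageSystem holds the shared damage logic for lightsaber and other hits on the dummy, enemy AIs and Vader boss.
; CastToActorsDoDamage runs a cast chain over those classes, sets IsSaber on the match and calls its TakeDamage.
; The library-style TakeDamage function plays a hit marker, subtracts fixed damage (higher for sabers) when allowed, and returns new health and death state.
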(fn TakeDamage
  (params (CanTakeDamage? :type Boolean) (Health :type Float%20%28single-precision%29) (HitMarker :type Sound%20Base%20Object%20Reference) (IsSaber? :type Boolean))
  (bind _returnvalue (select IsSaber? 4e+01 2e+01))
  (bind _returnvalue_2 (- Health _returnvalue))
  (if CanTakeDamage?
    (if IsSaber?
      (Audio|PlaySound2D 0 HitMarker 1.0 1.0 0.0 0 0)
      (else
        (Audio|PlaySound2D 0 HitMarker 1.0 1.0 0.0 0 0)
        (Development|PrintString 0 "Hit")))
    (if (<= _returnvalue_2 0.0)
      (return true 0.0)
      (else
        (return false _returnvalue_2)))))

(fn CasttoActors&DoDamage
  (params (Saber? :type Boolean) (HitActor :type Actor%20Object%20Reference))
  (bind _asbp_dummy (Utilities|Casting|CastToBP_Dummy HitActor)
    (:then
      (Variables|/Game/Lightsaber/Blueprints/MiscObjects/BP_Dummy.BP_Dummy_C|SetIsSaber? _asbp_dummy Saber?)
      (Default|TakeDamage _asbp_dummy)
      (return _asbp_dummy))
    (:CastFailed
      (bind _asbp_berserker_ai (Utilities|Casting|CastToBP_BerserkerAI HitActor)
        (:then
          (Variables|/Game/Lightsaber/Blueprints/AI_NPCs/BP_BerserkerAI.BP_BerserkerAI_C|SetIsSaber? _asbp_berserker_ai Saber?)
          (Default|TakeDamage _asbp_berserker_ai)
          (return _asbp_berserker_ai))
        (:CastFailed
          (bind _asbp_bxai (Utilities|Casting|CastToBP_BXAI HitActor)
            (:then
              (Variables|/Game/Lightsaber/Blueprints/AI_NPCs/BP_BXAI.BP_BXAI_C|SetIsSaber? _asbp_bxai Saber?)
              (Default|TakeDamage _asbp_bxai)
              (return _asbp_bxai))
            (:CastFailed
              (bind _asbp_clone_ai (Utilities|Casting|CastToBP_CloneAI HitActor)
                (:then
                  (Variables|/Game/Lightsaber/Blueprints/AI_NPCs/BP_CloneAI.BP_CloneAI_C|SetIsSaber? _asbp_clone_ai Saber?)
                  (Default|TakeDamage _asbp_clone_ai)
                  (return _asbp_clone_ai))
                (:CastFailed
                  (bind _asbp_vader_bossai (Utilities|Casting|CastToBP_VaderBOSSAI HitActor))
                  (Variables|/Game/Lightsaber/Blueprints/AI_NPCs/Bosses/BP_VaderBOSSAI.BP_VaderBOSSAI_C|SetIsSaber? _asbp_vader_bossai Saber?)
                  (Default|TakeDamage _asbp_vader_bossai)
                  (return _asbp_vader_bossai))))))))))