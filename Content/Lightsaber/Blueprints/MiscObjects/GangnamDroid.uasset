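; GangnamDroid is a damageable droid actor in the Lightsaber game that exposes its Sphere's location as a target point.
; TakeDamage passes health, a saber flag and a random hit marker to a nested TakeDamage call, then stores the new health.
; On death it spawns an explosion, plays a random death animation, disables damage and removes its Box.
; After a short delay it spawns a smoke burst and destroys itself.
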(event Custom|DeathSequence
  (bind _sphere (Variables|Default|GetSphere))
  (bind _returnvalue (Transformation|GetWorldLocation _sphere))
  (Development|PrintString "Dead")
  (Effects|SpawnEmitteratLocation "/Game/StarterContent/Particles/P_Explosion.P_Explosion" _returnvalue)
  (bind _item (Utilities|RandomItem (Variables|Default|GetDeathAnims))
    (:Get
      (Components|Animation|PlayAnimation (Variables|Default|GetSkeletalMesh) _item false)
      (Variables|Default|SetCanTakeDamage? false)
      (Components|DestroyComponent (Variables|Default|GetBox))
      (Utilities|FlowControl|Delay 3.0)
      (Effects|SpawnEmitteratLocation "/Game/StarterContent/Particles/SmokeBurst.SmokeBurst" _returnvalue)
      (Actor|DestroyActor))))

(event EventBeginPlay)

(event EventTick
  (params (DeltaSeconds :type Float%20%28single-precision%29)))

(event Collision|EventActorBeginOverlap
  (params (OtherActor :type Actor%20Object%20Reference)))

(fn ConstructionScript)

(fn TakeDamage
  (bind _item (Utilities|RandomItem (Variables|Default|GetHitMarkers))
    (:Get
      (bind (_isdead _newhealth) (CallFunction|TakeDamage (Variables|Default|GetCanTakeDamage?) (Variables|Default|GetHealth) _item (Variables|Default|GetIsSaber?)))
      (Variables|Default|SetHealth _newhealth)
      (if _isdead
        (CallFunction|DeathSequence)))))

(fn GetTarget
  (return (Transformation|GetWorldLocation (Variables|Default|GetSphere))))