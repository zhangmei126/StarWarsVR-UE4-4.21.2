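; Throwable thermal detonator prop for a lightsaber game, which can be picked up into a hand socket, dropped with physics, or optionally force-grabbed.
; A trigger press starts a delayed countdown of rising-pitch beeps with glow intensity changes, ending in an explosion effect and sound, with no damage logic.
; Overlapping a saber actor instead destroys it immediately with sparks and an impact sound, without exploding.
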(event OnComponentBeginOverlap(Detonator)
  (params (OverlappedComponent :type Primitive%20Component%20Object%20Reference) (OtherActor :type Actor%20Object%20Reference) (OtherComp :type Primitive%20Component%20Object%20Reference) (OtherBodyIndex :type Integer) (bFromSweep :type Boolean) (SweepResult :type Hit%20Result%20Structure%20%28by%20ref%29))
  (Utilities|Casting|CastToBP_SaberBase OtherActor)
  (CallFunction|Destroy))

(event Custom|DetonationSequence
  (bind _boom (Variables|Default|GetBoom))
  (bind _detonator (Variables|Default|GetDetonator))
  (bind _returnvalue (Transformation|GetWorldLocation _detonator))
  (Audio|PlaySoundatLocation "/Game/BF2_Assets/MiscWeapons/TermalDetonators/sounds/DetonatorActivate.DetonatorActivate" _returnvalue "0, 0, 0" 1.0 1.0 0.0 0 0 0)
  (Utilities|FlowControl|Delay 1.0)
  (CallFunction|BeepFn 1.0)
  (Utilities|FlowControl|Delay 1.0)
  (CallFunction|BeepFn 1.1)
  (Utilities|FlowControl|Delay 1.0)
  (CallFunction|BeepFn 1.2)
  (Utilities|FlowControl|Delay 1.0)
  (CallFunction|BeepFn 1.3)
  (Utilities|FlowControl|Delay 1.0)
  (Effects|SpawnEmitteratLocation "/Game/M5VFXVOL2/Particles/Explosion/Fire_Exp_00.Fire_Exp_00" _returnvalue "0, 0, 0" "0.600000,0.600000,0.600000")
  (Components|DestroyComponent (Variables|Default|GetDetonator))
  (Audio|Components|Audio|Play _boom 0.0)
  (if (not (Audio|Components|Audio|IsPlaying _boom))
    (Actor|DestroyActor)))

(event Custom|Destroy
  (bind _detonator (Variables|Default|GetDetonator))
  (bind _returnvalue (Transformation|GetWorldLocation _detonator))
  (Effects|SpawnEmitteratLocation "/Game/Lightsaber/Effects/P_Sparks.P_Sparks" _returnvalue)
  (Audio|PlaySoundatLocation "/Game/Lightsaber/Sound/SaberSounds/sw02_weapons_lightsaber_impacts_tonal_var_01_Cue.sw02_weapons_lightsaber_impacts_tonal_var_01_Cue" _returnvalue "0, 0, 0" 1.0 1.0 0.0 0 0 0)
  (Actor|DestroyActor))

(event EventTriggerPress
  (CallFunction|DetonationSequence))

(event EventPickup
  (params (Hand :type BP%20Motion%20Controller%20Object%20Reference))
  (bind _detonator (Variables|Default|GetDetonator))
  (Physics|SetSimulatePhysics _detonator false)
  (Transformation|AttachComponentToComponent _detonator (Variables|/Game/Lightsaber/Blueprints/BP_MotionController.BP_MotionController_C|GetHandMesh Hand) "ThermDet" "SnapToTarget" "SnapToTarget" "KeepWorld" true))

(event EventDrop
  (params (Hand :type BP%20Motion%20Controller%20Object%20Reference))
  (Physics|SetSimulatePhysics (Variables|Default|GetDetonator) true)
  (Transformation|DetachFromComponent (Variables|Default|GetDetonator) "KeepWorld" "KeepWorld" "KeepWorld" true))

(event EventForceGrab
  (params (Hand :type BP%20Motion%20Controller%20Object%20Reference))
  (if (Variables|Default|GetenableForceGrab)
    (Utilities|BasicForceGrab Hand (Variables|Default|GetDetonator))))

(fn ConstructionScript
  (Physics|SetSimulatePhysics (Variables|Default|GetDetonator) true))

(fn BeepFn
  (params (Pitch :type Float%20%28single-precision%29))
  (bind _beep (Variables|Default|GetBeep))
  (bind _glow (Variables|Default|GetGlow))
  (Audio|Components|Audio|SetPitchMultiplier _beep Pitch)
  (Audio|Components|Audio|Play _beep 0.0)
  (Rendering|Components|Light|SetIntensity _glow (Math|Interpolation|FInterpTo 5.0 5e+01 (Utilities|Time|GetWorldDeltaSeconds) 0.5))
  (Rendering|Components|Light|SetIntensity _glow (Math|Interpolation|FInterpTo 5e+01 5.0 (Utilities|Time|GetWorldDeltaSeconds) 0.5)))

(fn GetParent
  (return (Transformation|GetAttachParent (Variables|Default|GetDetonator))))