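; BP_Turret is an actor that automatically fires BP_LaserBullet projectiles at random intervals.
; BeginPlay starts a one-shot timer on Shoot, which re-arms it with a new random delay after each shot.
; Bullets spawn at the Arrow with slight random spread, inheriting the turret's size, color, velocity and optional muting.
; The construction script offsets the Arrow forward according to bullet length and collision multiplier.
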(event Custom|Shoot
  (bind _arrow (Variables|Default|GetArrow))
  (bind _returnvalue (Game|SpawnActorfromClass "/Game/Lightsaber/Blueprints/BP_LaserBullet.BP_LaserBullet_C" (Math|Transform|MakeTransform (Transformation|GetWorldLocation _arrow) (Math|Conversions|RotationFromXVector (+ (Math|Vector|GetForwardVector _arrow) (/ (Math|Random|RandomUnitVector) 75.0)))) "Undefined" 0 (Variables|Default|Getwidth) (Variables|Default|Getlength) (Variables|Default|GetcollisionMult) (Variables|Default|GetLaserColor) (Variables|Default|Getvelocity) 0))
  (if (Variables|Default|GetCan%20Play%20Sound?)
    _
    (else
      (Variables|/Game/Lightsaber/Blueprints/BP_LaserBullet.BP_LaserBullet_C|SetCanPlaySound _returnvalue false)))
  (Utilities|Time|SetTimerbyEvent (delegate Custom|Shoot) (Math|Random|RandomFloatinRange (Variables|Default|GetminDelay) (Variables|Default|GetmaxDelay))))

(event EventBeginPlay
  (Utilities|Time|SetTimerbyEvent (delegate Custom|Shoot) (Math|Random|RandomFloatinRange (Variables|Default|GetminDelay) (Variables|Default|GetmaxDelay))))

(fn ConstructionScript
  (Transformation|SetRelativeLocation (Variables|Default|GetArrow) (Math|Vector|MakeVector (* (Variables|Default|Getlength) (Variables|Default|GetcollisionMult) 4e+01) 0.0 125.0) false false))