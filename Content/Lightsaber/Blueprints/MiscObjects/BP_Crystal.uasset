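; BP_Crystal is a glowing lightsaber-game crystal prop that can be picked up, dropped and optionally Force-grabbed by a hand.
; Pickup turns off physics and snaps the mesh to the hand's Hilt socket, while Drop detaches it and restores physics.
; The construction script applies one Color to a dynamic material and point light, and gives the crystal a random non-uniform scale.
; GetParent returns the crystal's attach parent.
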(event EventPickup
  (params (Hand :type BP%20Motion%20Controller%20Object%20Reference))
  (bind _crystal (Variables|Default|Getcrystal))
  (Physics|SetSimulatePhysics _crystal false)
  (Transformation|AttachComponentToComponent _crystal (Variables|/Game/Lightsaber/Blueprints/BP_MotionController.BP_MotionController_C|GetHandMesh Hand) "Hilt" "SnapToTarget" "SnapToTarget" "KeepWorld" true))

(event EventDrop
  (params (Hand :type BP%20Motion%20Controller%20Object%20Reference))
  (Physics|SetSimulatePhysics (Variables|Default|Getcrystal) true)
  (Transformation|DetachFromComponent (Variables|Default|Getcrystal) "KeepWorld" "KeepWorld" "KeepWorld" true))

(event EventForceGrab
  (params (Hand :type BP%20Motion%20Controller%20Object%20Reference))
  (if (Variables|Default|GetenableForceGrab)
    (Utilities|BasicForceGrab Hand (Variables|Default|Getcrystal))))

(fn ConstructionScript
  (bind _color (Variables|Default|Getcolor))
  (bind _returnvalue (Rendering|Material|CreateDynamicMaterialInstance (Variables|Default|Getcrystal) 0 "/Game/Lightsaber/Models/Lightsaber/M_Crystal.M_Crystal" "None" :!class /Script/Engine.PrimitiveComponent))
  (Rendering|Material|SetVectorParameterValue _returnvalue "Color" _color :!class /Script/Engine.MaterialInstanceDynamic)
  (Rendering|Components|Light|SetLightColor (Variables|Default|GetPointLight) _color true)
  (Transformation|SetWorldScale3D (Variables|Default|Getcrystal) (Math|Vector|MakeVector (Math|Random|RandomFloatinRange 0.1 0.25) (Math|Random|RandomFloatinRange 0.1 0.25) (Math|Random|RandomFloatinRange 0.1 0.25))))

(fn GetParent
  (return (Transformation|GetAttachParent (Variables|Default|Getcrystal))))