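; BXToy is a grabbable BX figure prop in a lightsaber game with hand-based pickup.
; Pickup disables physics and snaps the figure to the hand mesh's Hilt socket, while Drop re-enables physics and detaches it in place.
; ForceGrab calls the shared BasicForceGrab on the figure when force grabbing is enabled, and GetParent reports what the figure is attached to.
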(event EventPickup
  (params (Hand :type BP%20Motion%20Controller%20Object%20Reference))
  (bind _bxfigure (Variables|Default|GetBXFigure))
  (Physics|SetSimulatePhysics _bxfigure false)
  (Transformation|AttachComponentToComponent _bxfigure (Variables|/Game/Lightsaber/Blueprints/BP_MotionController.BP_MotionController_C|GetHandMesh Hand) "Hilt" "SnapToTarget" "SnapToTarget" "KeepWorld" true))

(event EventDrop
  (params (Hand :type BP%20Motion%20Controller%20Object%20Reference))
  (bind _bxfigure (Variables|Default|GetBXFigure))
  (Physics|SetSimulatePhysics _bxfigure true)
  (Transformation|DetachFromComponent _bxfigure "KeepWorld" "KeepWorld" "KeepWorld" true))

(event EventForceGrab
  (params (Hand :type BP%20Motion%20Controller%20Object%20Reference))
  (if (Variables|Default|GetenableForceGrab)
    (Utilities|BasicForceGrab Hand (Variables|Default|GetBXFigure))))

(fn ConstructionScript)

(fn GetParent
  (return (Transformation|GetAttachParent (Variables|Default|GetBXFigure))))