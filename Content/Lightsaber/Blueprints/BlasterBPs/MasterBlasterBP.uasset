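; Base blaster pistol Blueprint that can be picked up, dropped, force-grabbed and fired by a hand.
; Pickup snaps the Gun component to a socket on the hand mesh and disables physics, while drop detaches it and re-enables physics.
; Trigger press spawns a colored BP_LaserBullet at the Arrow's transform and plays a fire sound at the gun.
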(event Custom|Shoot
  (bind _arrow (Variables|Default|GetArrow))
  (Game|SpawnActorfromClass "/Game/Lightsaber/Blueprints/BP_LaserBullet.BP_LaserBullet_C" (Math|Transform|MakeTransform (Transformation|GetWorldLocation _arrow) (Transformation|GetWorldRotation _arrow)) "Undefined" 0 2.0 1.5 1.5 (Variables|Default|GetColor) 3e+03 0)
  (Audio|PlaySoundatLocation (Variables|Default|GetFireSound) (Transformation|GetWorldLocation (Variables|Default|GetGun)) "0, 0, 0" 1.0 1.0 0.0 0 0 0))

(event EventTick
  (params (DeltaSeconds :type Float%20%28single-precision%29)))

(event EventPickup
  (params (Hand :type BP%20Motion%20Controller%20Object%20Reference))
  (Transformation|AttachComponentToComponent (Variables|Default|GetGun) (Variables|/Game/Lightsaber/Blueprints/BP_MotionController.BP_MotionController_C|GetHandMesh Hand) (Variables|Default|GetAttachedSocketName) "SnapToTarget" "SnapToTarget" "KeepWorld" true)
  (Physics|SetSimulatePhysics (Variables|Default|GetGun) false))

(event EventDrop
  (params (Hand :type BP%20Motion%20Controller%20Object%20Reference))
  (Transformation|DetachFromComponent (Variables|Default|GetGun) "KeepWorld" "KeepWorld" "KeepWorld" true)
  (Physics|SetSimulatePhysics (Variables|Default|GetGun) true))

(event EventForceGrab
  (params (Hand :type BP%20Motion%20Controller%20Object%20Reference))
  (Utilities|BasicForceGrab Hand (Variables|Default|GetGun)))

(event EventTriggerPress
  (CallFunction|Shoot))

(fn ConstructionScript)

(fn GetParent
  (return (Transformation|GetAttachParent (Variables|Default|GetGun))))