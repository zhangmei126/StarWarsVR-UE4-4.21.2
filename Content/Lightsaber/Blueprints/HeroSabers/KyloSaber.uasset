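; Kylo Ren-style crossguard lightsaber that drives a main blade and two guard blades as child sabers.
; Turn on, turn off, toggle and crystal color events are forwarded to all three blades, with powering on and toggling gated by an optional crystal requirement.
; The construction script passes base color and sounds to the guards and hides their lights, which Tick also re-hides every frame.
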(event EventBeginPlay
  (|CallParentFunction) ; This node is disabled and will not be called.\nDrag off pins to build functionality.
)

(event Collision|EventActorBeginOverlap
  (params (OtherActor :type Actor%20Object%20Reference)))

(event EventUseCrystal
  (params (Crystal :type BP%20Crystal%20Object%20Reference))
  (bind _color (Variables|/Game/Lightsaber/Blueprints/MiscObjects/BP_Crystal.BP_Crystal_C|Getcolor Crystal))
  (Variables|Default|SethasCrystal true)
  (Default|SetColor (CallFunction|GetChildSaber (Variables|Default|GetSaber)) _color)
  (Default|SetColor (CallFunction|GetChildSaber (Variables|Default|GetSaberGuard1)) _color)
  (Default|SetColor (CallFunction|GetChildSaber (Variables|Default|GetSaberGuard2)) _color))

(event EventFaceButton1Press
  (if (or (Variables|Default|GethasCrystal) (not (Variables|Default|GetrequireCrystal)))
    (Default|TurnToggle (CallFunction|GetChildSaber (Variables|Default|GetSaber)))
    (Default|TurnToggle (CallFunction|GetChildSaber (Variables|Default|GetSaberGuard1)))
    (Default|TurnToggle (CallFunction|GetChildSaber (Variables|Default|GetSaberGuard2)))))

(event EventTurnon
  (if (or (Variables|Default|GethasCrystal) (not (Variables|Default|GetrequireCrystal)))
    (Default|Turnon (CallFunction|GetChildSaber (Variables|Default|GetSaber)))
    (Default|Turnon (CallFunction|GetChildSaber (Variables|Default|GetSaberGuard1)))
    (Default|Turnon (CallFunction|GetChildSaber (Variables|Default|GetSaberGuard2)))))

(event EventTurnOff
  (Default|TurnOff (CallFunction|GetChildSaber (Variables|Default|GetSaber)))
  (Default|TurnOff (CallFunction|GetChildSaber (Variables|Default|GetSaberGuard1)))
  (Default|TurnOff (CallFunction|GetChildSaber (Variables|Default|GetSaberGuard2))))

(event EventTick
  (params (DeltaSeconds :type Float%20%28single-precision%29))
  (bind _saberguard1 (Variables|Default|GetSaberGuard1))
  (bind _saberguard2 (Variables|Default|GetSaberGuard2))
  (bind _saber (CallFunction|GetChildSaber _saberguard2))
  (bind _saber_2 (CallFunction|GetChildSaber _saberguard1))
  (Rendering|SetVisibility (Variables|/Game/Lightsaber/Blueprints/BP_SaberBase.BP_SaberBase_C|GetBaseLight _saber_2) false false)
  (Rendering|SetVisibility (Variables|/Game/Lightsaber/Blueprints/BP_SaberBase.BP_SaberBase_C|GetEndLight _saber_2) false false)
  (Rendering|SetVisibility (Variables|/Game/Lightsaber/Blueprints/BP_SaberBase.BP_SaberBase_C|GetBaseLight _saber) false false)
  (Rendering|SetVisibility (Variables|/Game/Lightsaber/Blueprints/BP_SaberBase.BP_SaberBase_C|GetEndLight _saber) false false))

(fn ConstructionScript
  (bind _basecolor (Variables|Default|GetbaseColor))
  (bind _saberguard1 (Variables|Default|GetSaberGuard1))
  (bind _saberguard2 (Variables|Default|GetSaberGuard2))
  (bind _saber (CallFunction|GetChildSaber _saberguard2))
  (bind _saber_2 (CallFunction|GetChildSaber _saberguard1))
  (|CallParentFunction)
  (Default|SetColor _saber_2 _basecolor)
  (Default|SetColor _saber _basecolor)
  (Rendering|SetVisibility (Variables|/Game/Lightsaber/Blueprints/BP_SaberBase.BP_SaberBase_C|GetBaseLight _saber_2) false false)
  (Rendering|SetVisibility (Variables|/Game/Lightsaber/Blueprints/BP_SaberBase.BP_SaberBase_C|GetEndLight _saber_2) false false)
  (Rendering|SetVisibility (Variables|/Game/Lightsaber/Blueprints/BP_SaberBase.BP_SaberBase_C|GetBaseLight _saber) false false)
  (Rendering|SetVisibility (Variables|/Game/Lightsaber/Blueprints/BP_SaberBase.BP_SaberBase_C|GetEndLight _saber) false false)
  (Variables|/Game/Lightsaber/Blueprints/BP_SaberBase.BP_SaberBase_C|SetactivateSound _saber_2 (Variables|Default|GetActivateSound))
  (Variables|/Game/Lightsaber/Blueprints/BP_SaberBase.BP_SaberBase_C|SetdeactivateSound _saber_2 (Variables|Default|GetDeactivateSound))
  (Variables|/Game/Lightsaber/Blueprints/BP_SaberBase.BP_SaberBase_C|SetIdleSoundSource _saber_2 (Variables|Default|GetActiveSound))
  (Variables|/Game/Lightsaber/Blueprints/BP_SaberBase.BP_SaberBase_C|SetactivateSound _saber (Variables|Default|GetActivateSound))
  (Variables|/Game/Lightsaber/Blueprints/BP_SaberBase.BP_SaberBase_C|SetdeactivateSound _saber (Variables|Default|GetDeactivateSound))
  (Variables|/Game/Lightsaber/Blueprints/BP_SaberBase.BP_SaberBase_C|SetIdleSoundSource _saber (Variables|Default|GetActiveSound)))