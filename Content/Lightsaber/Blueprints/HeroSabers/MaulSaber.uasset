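; MaulSaber is a hero lightsaber Blueprint that controls a child saber, Saber2, on top of its parent saber class.
; At BeginPlay it copies its activate, deactivate and idle sounds to Saber2, and the construction script applies the base color.
; Face button 2 toggles Saber2 while the trigger is pressed, subject to any crystal requirement.
; Using a crystal recolors Saber2; the TurnOff and Turnon events are empty.
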(event Custom|UseCrystal
  (params (Crystal :type BP%20Crystal%20Object%20Reference))
  (Variables|Default|SethasCrystal true)
  (Default|SetColor (CallFunction|GetChildSaber (Variables|Default|GetSaber2)) (Variables|/Game/Lightsaber/Blueprints/MiscObjects/BP_Crystal.BP_Crystal_C|Getcolor Crystal)))

(event EventBeginPlay
  (bind _saber2 (Variables|Default|GetSaber2))
  (bind _saber (CallFunction|GetChildSaber _saber2))
  (|CallParentFunction)
  (Variables|/Game/Lightsaber/Blueprints/BP_SaberBase.BP_SaberBase_C|SetactivateSound _saber (Variables|Default|GetActivateSound))
  (Variables|/Game/Lightsaber/Blueprints/BP_SaberBase.BP_SaberBase_C|SetdeactivateSound _saber (Variables|Default|GetDeactivateSound))
  (Variables|/Game/Lightsaber/Blueprints/BP_SaberBase.BP_SaberBase_C|SetIdleSoundSource _saber (Variables|Default|GetActiveSound)))

(event Collision|EventActorBeginOverlap
  (params (OtherActor :type Actor%20Object%20Reference)))

(event EventTick
  (params (DeltaSeconds :type Float%20%28single-precision%29)))

(event EventFaceButton2Press
  (if (and (or (Variables|Default|GethasCrystal) (not (Variables|Default|GetrequireCrystal))) (Variables|Default|GetTriggerPressed?))
    (Default|TurnToggle (CallFunction|GetChildSaber (Variables|Default|GetSaber2)))))

(event EventTurnOff)

(event EventTurnon)

(fn ConstructionScript
  (|CallParentFunction)
  (Default|SetColor (CallFunction|GetChildSaber (Variables|Default|GetSaber2)) (Variables|Default|GetbaseColor)))