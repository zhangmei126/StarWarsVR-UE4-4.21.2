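; Kylo Ren crossguard lightsaber that can be picked up, force-grabbed and dropped, snapping to a hand socket and turning off on release.
; Three child-actor blades (main plus two handguards) are switched and colored together through a cast helper.
; An overlapping crystal recolors all blades, is destroyed, and unlocks ignition when a crystal is required.
; Tick hides the handguard blades' base and end lights every frame.
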(event OnComponentBeginOverlap(CrystalCollision)
  (params (OverlappedComponent :type Primitive%20Component%20Object%20Reference) (OtherActor :type Actor%20Object%20Reference) (OtherComp :type Primitive%20Component%20Object%20Reference) (OtherBodyIndex :type Integer) (bFromSweep :type Boolean) (SweepResult :type Hit%20Result%20Structure%20%28by%20ref%29))
  (bind _asbp_crystal (Utilities|Casting|CastToBP_Crystal OtherActor))
  (CallFunction|UseCrystal _asbp_crystal)
  (Actor|DestroyActor _asbp_crystal))

(event Custom|TurnOn
  (if (or (Variables|Default|GethasCrystal) (not (Variables|Default|GetrequireCrystal)))
    (Default|Turnon (CallFunction|GetChildSaber (Variables|Default|GetSaber)))
    (Default|Turnon (CallFunction|GetChildSaber (Variables|Default|GetHandGuard1)))
    (Default|Turnon (CallFunction|GetChildSaber (Variables|Default|GetHandGuard2)))))

(event Custom|TurnOff
  (Default|TurnOff (CallFunction|GetChildSaber (Variables|Default|GetSaber)))
  (Default|TurnOff (CallFunction|GetChildSaber (Variables|Default|GetHandGuard1)))
  (Default|TurnOff (CallFunction|GetChildSaber (Variables|Default|GetHandGuard2))))

(event Custom|UseCrystal
  (params (Crystal :type BP%20Crystal%20Object%20Reference))
  (bind _color (Variables|/Game/Lightsaber/Blueprints/MiscObjects/BP_Crystal.BP_Crystal_C|Getcolor Crystal))
  (Variables|Default|SethasCrystal true)
  (Default|SetColor (CallFunction|GetChildSaber (Variables|Default|GetSaber)) _color)
  (Default|SetColor (CallFunction|GetChildSaber (Variables|Default|GetHandGuard1)) _color)
  (Default|SetColor (CallFunction|GetChildSaber (Variables|Default|GetHandGuard2)) _color))

(event EventTick
  (params (DeltaSeconds :type Float%20%28single-precision%29))
  (bind _handguard1 (Variables|Default|GetHandGuard1))
  (bind _handguard2 (Variables|Default|GetHandGuard2))
  (bind _saber (CallFunction|GetChildSaber _handguard2))
  (bind _saber_2 (CallFunction|GetChildSaber _handguard1))
  (Rendering|SetVisibility (Variables|/Game/Lightsaber/Blueprints/CustomBladeClasses/KyloRenSaberBlade.KyloRenSaberBlade_C|GetEndLight _saber_2) false false)
  (Rendering|SetVisibility (Variables|/Game/Lightsaber/Blueprints/CustomBladeClasses/KyloRenSaberBlade.KyloRenSaberBlade_C|GetBaseLight _saber_2) false false)
  (Rendering|SetVisibility (Variables|/Game/Lightsaber/Blueprints/CustomBladeClasses/KyloRenSaberBlade.KyloRenSaberBlade_C|GetBaseLight _saber) false false)
  (Rendering|SetVisibility (Variables|/Game/Lightsaber/Blueprints/CustomBladeClasses/KyloRenSaberBlade.KyloRenSaberBlade_C|GetEndLight _saber) false false))

(event EventPickup
  (params (Hand :type BP%20Motion%20Controller%20Object%20Reference))
  (Variables|Default|SetHand Hand)
  (Transformation|AttachComponentToComponent (Variables|Default|GetHilt) (Variables|/Game/Lightsaber/Blueprints/BP_MotionController.BP_MotionController_C|GetHandMesh Hand) "KyloSaber" "SnapToTarget" "SnapToTarget" "KeepWorld" true)
  (Physics|SetSimulatePhysics (Variables|Default|GetHilt) false))

(event EventForceGrab
  (params (Hand :type BP%20Motion%20Controller%20Object%20Reference))
  (if (Variables|Default|GetenableForceGrab)
    (Utilities|BasicForceGrab Hand (Variables|Default|GetHilt))))

(event EventDrop
  (params (Hand :type BP%20Motion%20Controller%20Object%20Reference))
  (Transformation|DetachFromComponent (Variables|Default|GetHilt) "KeepWorld" "KeepWorld" "KeepWorld" true)
  (Physics|SetSimulatePhysics (Variables|Default|GetHilt) (Variables|Default|GetsimulatePhysics))
  (CallFunction|TurnOff))

(event EventBeginPlay
  (Physics|SetSimulatePhysics (Variables|Default|GetHilt) (Variables|Default|GetsimulatePhysics)))

(event EventFaceButton1Press
  (if (or (Variables|Default|GethasCrystal) (not (Variables|Default|GetrequireCrystal)))
    (Default|TurnToggle (CallFunction|GetChildSaber (Variables|Default|GetSaber)))
    (Default|TurnToggle (CallFunction|GetChildSaber (Variables|Default|GetHandGuard1)))
    (Default|TurnToggle (CallFunction|GetChildSaber (Variables|Default|GetHandGuard2)))))

(fn ConstructionScript
  (bind _basecolor (Variables|Default|GetbaseColor))
  (|CallParentFunction)
  (Default|SetColor (CallFunction|GetChildSaber (Variables|Default|GetSaber)) _basecolor)
  (Default|SetColor (CallFunction|GetChildSaber (Variables|Default|GetHandGuard1)) _basecolor)
  (Default|SetColor (CallFunction|GetChildSaber (Variables|Default|GetHandGuard2)) _basecolor))

(fn GetChildSaber
  (params (ChildActor :type Child%20Actor%20Component%20Object%20Reference))
  (if true
    (bind _askylo_ren_saber_blade (Utilities|Casting|CastToKyloRenSaberBlade (Variables|/Script/Engine.ChildActorComponent|GetChildActor ChildActor)))
    (return _askylo_ren_saber_blade)))

(fn GetParent
  (return (Transformation|GetAttachParent (Variables|Default|GetHilt))))