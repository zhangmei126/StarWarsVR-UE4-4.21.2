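; Base VR hero lightsaber: a physics hilt that can be picked up, dropped or force-grabbed, driving a child BP_SaberBase blade.
; Pickup attaches the hilt to the hand; a second controller overlapping the grip aims it via look-at rotation, taking roll from that hand.
; Trigger plus face button toggles the blade, optionally requiring a crystal, which recolors it and is consumed on overlap.
; Construction passes base color and sounds to the blade.
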(event OnComponentBeginOverlap(CrystalCollision)
  (params (OverlappedComponent :type Primitive%20Component%20Object%20Reference) (OtherActor :type Actor%20Object%20Reference) (OtherComp :type Primitive%20Component%20Object%20Reference) (OtherBodyIndex :type Integer) (bFromSweep :type Boolean) (SweepResult :type Hit%20Result%20Structure%20%28by%20ref%29))
  (bind _asbp_crystal (Utilities|Casting|CastToBP_Crystal OtherActor))
  (CallFunction|UseCrystal _asbp_crystal)
  (Actor|DestroyActor _asbp_crystal))

(event OnComponentBeginOverlap(SecondHandCollision)
  (params (OverlappedComponent :type Primitive%20Component%20Object%20Reference) (OtherActor :type Actor%20Object%20Reference) (OtherComp :type Primitive%20Component%20Object%20Reference) (OtherBodyIndex :type Integer) (bFromSweep :type Boolean) (SweepResult :type Hit%20Result%20Structure%20%28by%20ref%29))
  (if (Variables|Default|GetFirstHandAttached?)
    (bind _asbp_motion_controller (Utilities|Casting|CastToBP_MotionController OtherActor))
    (if (!= (Variables|/Game/Lightsaber/Blueprints/BP_MotionController.BP_MotionController_C|GetMotionController _asbp_motion_controller) (Variables|Default|GetFirstHand))
      (Variables|Default|SetIsSecondHandTrackingActive? true)
      (Variables|Default|SetSecondHand (Variables|/Game/Lightsaber/Blueprints/BP_MotionController.BP_MotionController_C|GetMotionController _asbp_motion_controller)))))

(event OnComponentEndOverlap(SecondHandCollision)
  (params (OverlappedComponent :type Primitive%20Component%20Object%20Reference) (OtherActor :type Actor%20Object%20Reference) (OtherComp :type Primitive%20Component%20Object%20Reference) (OtherBodyIndex :type Integer))
  (if (Variables|Default|GetIsSecondHandTrackingActive?)
    (Utilities|IsValid (Variables|Default|GetSecondHand)
      (:Is%20Valid
        (if (and (.bSuccess (Utilities|Casting|CastToBP_MotionController (Components|GetOwner (Variables|Default|GetSecondHand)))) (Utilities|Enum|NotEqual(Enum) (Variables|/Game/Lightsaber/Blueprints/BP_MotionController.BP_MotionController_C|GetGripState (.AsBP%20Motion%20Controller (Utilities|Casting|CastToBP_MotionController (Components|GetOwner (Variables|Default|GetSecondHand))))) "NewEnumerator2"))
          (Variables|Default|SetIsSecondHandTrackingActive? false :!label _label)
          (Variables|Default|SetSecondHand 0)
          (Transformation|SetRelativeRotation (Variables|Default|GetHilt) (Variables|Default|GetOneHandedRotation) false false)))
      (:Is%20Not%20Valid
        (goto _label)))))

(event Custom|TurnOn
  (if (or (Variables|Default|GethasCrystal) (not (Variables|Default|GetrequireCrystal)))
    (Default|Turnon (CallFunction|GetChildSaber (Variables|Default|GetSaber)))))

(event Custom|TurnToggle
  (Default|TurnToggle (CallFunction|GetChildSaber (Variables|Default|GetSaber))))

(event Custom|TurnOff
  (Default|TurnOff (CallFunction|GetChildSaber (Variables|Default|GetSaber))))

(event Custom|UseCrystal
  (params (Crystal :type BP%20Crystal%20Object%20Reference))
  (Variables|Default|SethasCrystal true)
  (Default|SetColor (CallFunction|GetChildSaber (Variables|Default|GetSaber)) (Variables|/Game/Lightsaber/Blueprints/MiscObjects/BP_Crystal.BP_Crystal_C|Getcolor Crystal)))

(event EventTick
  (params (DeltaSeconds :type Float%20%28single-precision%29))
  (bind _firsthand (Variables|Default|GetFirstHand))
  (bind _secondhand (Variables|Default|GetSecondHand))
  (bind _returnvalue (Transformation|GetWorldLocation _firsthand))
  (bind _returnvalue_2 (Transformation|GetWorldLocation _secondhand))
  (bind _returnvalue_3 (Math|Rotator|FindLookatRotation _returnvalue _returnvalue_2))
  (bind (_roll _pitch _yaw) (Math|Rotator|BreakRotator _returnvalue_3))
  (if (and (Variables|Default|GetIsSecondHandTrackingActive?) (Utilities|IsValid (Variables|Default|GetSecondHand)))
    (Transformation|SetWorldRotation (Variables|Default|GetHilt) (Math|Rotator|MakeRotator (.Roll (Math|Rotator|BreakRotator (Transformation|GetWorldRotation _secondhand))) _pitch _yaw) false false)
    (bind _asbp_saber_base (Utilities|Casting|CastToBP_SaberBase (Variables|/Script/Engine.ChildActorComponent|GetChildActor (Variables|Default|GetSaber))))
    (Variables|Default|SetIsActive? (Variables|/Game/Lightsaber/Blueprints/BP_SaberBase.BP_SaberBase_C|GetisActive _asbp_saber_base))))

(event EventPickup
  (params (Hand :type BP%20Motion%20Controller%20Object%20Reference))
  (if (not (Variables|Default|GetFirstHandAttached?))
    (bind _asbp_motion_controller (Utilities|Casting|CastToBP_MotionController Hand))
    (Variables|Default|SetHand Hand)
    (Transformation|AttachComponentToComponent (Variables|Default|GetHilt) (Variables|/Game/Lightsaber/Blueprints/BP_MotionController.BP_MotionController_C|GetHandMesh Hand) (Variables|Default|GetAttachedSocketName) "SnapToTarget" "SnapToTarget" "KeepWorld" true)
    (Physics|SetSimulatePhysics (Variables|Default|GetHilt) false)
    (Transformation|SetRelativeRotation (Variables|Default|GetHilt) (Variables|Default|GetOneHandedRotation) false false)
    (Variables|Default|SetFirstHandAttached? true)
    (Variables|Default|SetIsSecondHandTrackingActive? false)
    (Variables|Default|SetFirstHand (Variables|/Game/Lightsaber/Blueprints/BP_MotionController.BP_MotionController_C|GetMotionController _asbp_motion_controller))))

(event EventTriggerPress
  (Variables|Default|SetTriggerPressed? true))

(event EventForceGrab
  (params (Hand :type BP%20Motion%20Controller%20Object%20Reference))
  (if (Variables|Default|GetenableForceGrab)
    (Utilities|BasicForceGrab Hand (Variables|Default|GetHilt))))

(event EventDrop
  (params (Hand :type BP%20Motion%20Controller%20Object%20Reference))
  (Transformation|DetachFromComponent (Variables|Default|GetHilt) "KeepWorld" "KeepWorld" "KeepWorld" true)
  (Physics|SetSimulatePhysics (Variables|Default|GetHilt) (Variables|Default|GetsimulatePhysics))
  (Variables|Default|SetFirstHandAttached? false)
  (Variables|Default|SetIsSecondHandTrackingActive? false)
  (if (Variables|Default|GetTurnOffOnDrop?)
    (CallFunction|TurnOff)))

(event EventTriggerRelease
  (Variables|Default|SetTriggerPressed? false))

(event EventBeginPlay
  (Physics|SetSimulatePhysics (Variables|Default|GetHilt) (Variables|Default|GetsimulatePhysics)))

(event EventFaceButton1Press
  (if (and (or (Variables|Default|GethasCrystal) (not (Variables|Default|GetrequireCrystal))) (Variables|Default|GetTriggerPressed?))
    (Default|TurnToggle (CallFunction|GetChildSaber (Variables|Default|GetSaber)))))

(fn ConstructionScript
  (bind _saber (Variables|Default|GetSaber))
  (bind _saber_2 (CallFunction|GetChildSaber _saber))
  (|CallParentFunction)
  (Default|SetColor (CallFunction|GetChildSaber (Variables|Default|GetSaber)) (Variables|Default|GetbaseColor))
  (Variables|/Game/Lightsaber/Blueprints/BP_SaberBase.BP_SaberBase_C|SetactivateSound _saber_2 (Variables|Default|GetActivateSound))
  (Variables|/Game/Lightsaber/Blueprints/BP_SaberBase.BP_SaberBase_C|SetdeactivateSound _saber_2 (Variables|Default|GetDeactivateSound))
  (Variables|/Game/Lightsaber/Blueprints/BP_SaberBase.BP_SaberBase_C|SetIdleSoundSource _saber_2 (Variables|Default|GetActiveSound)))

(fn GetChildSaber
  (params (ChildActor :type Child%20Actor%20Component%20Object%20Reference))
  (if true
    (bind _asbp_saber_base (Utilities|Casting|CastToBP_SaberBase (Variables|/Script/Engine.ChildActorComponent|GetChildActor ChildActor)))
    (return _asbp_saber_base)))

(fn GetParent
  (return (Transformation|GetAttachParent (Variables|Default|GetHilt))))