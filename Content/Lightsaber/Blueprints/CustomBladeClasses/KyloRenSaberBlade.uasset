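; Kylo Ren lightsaber blade actor that toggles on and off with sound, lights and collision, extending over an activation time.
; Each tick it updates blade scale, idle sound and movement delta.
; Line traces position the tip light and lay interpolated burn decals along surfaces, skipping Saber physical materials.
; GetDeflect optionally auto-aims deflections by sphere-tracing for BI_Targetable actors from saber, head or hand, otherwise using DeflectDir's forward vector.
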(event Custom|TurnOff
  ;[1 1 1] Turn on/off
  (if (Variables|Default|GetisActive)
    (Rendering|SetVisibility (Variables|Default|GetSaber) false false)
    (Collision|SetCollisionEnabled (Variables|Default|GetCollision) "NoCollision")
    (CallFunction|ForceInit)
    (CallFunction|PlaySound (Variables|Sounds|GetdeactivateSound))
    (Variables|Default|SetisActive false)))

(event Custom|SetColor
  (params (Color :type Linear%20Color%20Structure))
  ;[1 1 1] SetColor
  (Variables|Basic|SetColor Color)
  (Rendering|Material|SetVectorParameterValue (Variables|Default|GetSaberMat) "Color" (Variables|Basic|GetColor) :!class /Script/Engine.MaterialInstanceDynamic)
  (Rendering|Components|Light|SetLightColor (Variables|Default|GetEndLight) (Variables|Basic|GetColor) true))

(event Custom|ForceInit
  ;[1 1 1] Force
  (Variables|Default|SetlastSaberPos (Transformation|GetWorldLocation (Variables|Default|GetSaber)))
  (Variables|Default|SetlastForce "0, 0, 0"))

(event Custom|Init
  ;[1 1 1] Init
  (Rendering|SetVisibility (Variables|Default|GetSaber) false false)
  (Collision|SetCollisionEnabled (Variables|Default|GetCollision) "NoCollision")
  (CallFunction|ForceInit)
  (Variables|Default|SetisActive false))

(event Custom|ActivationTick
  (bind _width (Variables|Basic|GetWidth))
  (bind _saber (Variables|Default|GetSaber))
  (bind _width_2 (Variables|Basic|GetWidth))
  (bind _collisionmult (Variables|Basic|GetCollisionMult))
  (bind _returnvalue (/ _width 1e+02))
  (bind _returnvalue_2 (* _width_2 _collisionmult))
  (if (Variables|Default|GetisActive)
    (bind _output_get (Variables|Default|SetactivationTimer (Math|Float|Clamp(Float) (+ (Variables|Default|GetactivationTimer) (Utilities|Time|GetWorldDeltaSeconds)) 0.0 (Variables|Basic|GetactivationLength))))
    (Transformation|SetRelativeScale3D _saber (Math|Vector|MakeVector _returnvalue _returnvalue (/ (* (Variables|Basic|GetLength) (/ _output_get (Variables|Basic|GetactivationLength))) 1e+02)))
    (Transformation|SetRelativeLocation _saber (Math|Vector|MakeVector 0.0 0.0 (/ (* (Variables|Basic|GetLength) (/ _output_get (Variables|Basic|GetactivationLength))) 2.0)) false false)
    (Components|Box|SetBoxExtent (Variables|Default|GetCollision) (Math|Vector|MakeVector _returnvalue_2 _returnvalue_2 (/ (* (/ _output_get (Variables|Basic|GetactivationLength)) (Variables|Basic|GetLength)) 2.0)) true)
    (else
      (Variables|Default|SetactivationTimer 0.0))))

(event Custom|TurnToggle
  ;[1 1 1] Turn on/off
  (if (Variables|Default|GetisActive)
    (CallFunction|TurnOff)
    (else
      (CallFunction|Turnon))))

(event Custom|TurnOn
  ;[1 1 1] Turn on/off
  (if (not (Variables|Default|GetisActive))
    (Rendering|SetVisibility (Variables|Default|GetSaber) true false)
    (Collision|SetCollisionEnabled (Variables|Default|GetCollision) "QueryAndPhysics")
    (CallFunction|PlaySound (Variables|Sounds|GetactivateSound))
    (CallFunction|ActivationTick)
    (Variables|Default|SetisActive true)))

(event Custom|ForceTick
  (bind _saber (Variables|Default|GetSaber))
  (bind _returnvalue (Transformation|GetWorldLocation _saber))
  ;[1 1 1] Force
  (Variables|Default|SetlastForce (- _returnvalue (Variables|Default|GetlastSaberPos)))
  (Variables|Default|SetlastSaberPos _returnvalue))

(event Custom|DrawDecal
  (bind _pointer (Variables|Default|GetPointer))
  (bind _returnvalue (Transformation|GetWorldLocation _pointer))
  ;[1 1 1] Decal
  (if (and (Variables|Basic|GetenableDecal) (Variables|Default|GetisActive))
    (bind (_outhit _returnvalue_2) (Collision|LineTraceByChannel _returnvalue (+ _returnvalue (* (Math|Rotator|GetRotationXVector (Transformation|GetWorldRotation _pointer)) (- (Variables|Basic|GetLength) 5.0))) "TraceTypeQuery1" false 0 "None"))
    (if _returnvalue_2
      (if (Math|Vector|NotEqual(Vector) (Variables|Default|GetlastDecalLoc) "0, 0, 0" 0.0)
        (Utilities|FlowControl|Sequence
          (:then_0
            (for _index (range 0 (Math|Float|Ceil (/ (Math|Vector|VectorLength (- (.Location (Collision|BreakHitResult _outhit)) (Variables|Default|GetlastDecalLoc))) (/ (Variables|Basic|GetWidth) 2.0))))
              (if (Utilities|Enum|Equal(Enum) (Utilities|GetObjectName (Class|MaterialInterface|GetPhysicalMaterial (.ReturnValue (Class|PrimitiveComponent|GetMaterialfromCollisionFaceIndex (.HitComponent (Collision|BreakHitResult _outhit)))))) "None")
                (Utilities|SpawnLaserDecal (Math|Conversions|ToVector(Float) (* (Variables|Basic|GetWidth) 1.5)) (.HitComponent (Collision|BreakHitResult _outhit)) (+ (* (- (.Location (Collision|BreakHitResult _outhit)) (Variables|Default|GetlastDecalLoc)) (/ (Math|Conversions|ToFloat(Integer) _index) (Math|Conversions|ToFloat(Integer) (Math|Float|Ceil (/ (Math|Vector|VectorLength (- (.Location (Collision|BreakHitResult _outhit)) (Variables|Default|GetlastDecalLoc))) (/ (Variables|Basic|GetWidth) 2.0)))))) (Variables|Default|GetlastDecalLoc)) (.Normal (Collision|BreakHitResult _outhit)) :!label _label)
                (elif (not (Utilities|Enum|Equal(Enum) (Utilities|GetObjectName (Class|MaterialInterface|GetPhysicalMaterial (.ReturnValue (Class|PrimitiveComponent|GetMaterialfromCollisionFaceIndex (.HitComponent (Collision|BreakHitResult _outhit)))))) "Saber"))
                  (goto _label)))))
          (:then_1
            (Variables|Default|SetlastDecalLoc (.Location (Collision|BreakHitResult _outhit)) :!label _label_2)))
        (else
          (goto _label_2)))
      (else
        (Variables|Default|SetlastDecalLoc "0, 0, 0")))
    (else
      (Variables|Default|SetlastDecalLoc "0, 0, 0"))))

(event Custom|LightPos
  (bind _pointer (Variables|Default|GetPointer))
  (bind _returnvalue (Transformation|GetWorldLocation _pointer))
  ;[1 1 1] Light
  (if (Variables|Default|GetisActive)
    (bind (_outhit _returnvalue_2) (Collision|LineTraceByChannel _returnvalue (+ _returnvalue (* (Math|Rotator|GetRotationXVector (Transformation|GetWorldRotation _pointer)) (- (Variables|Basic|GetLength) 5.0))) "TraceTypeQuery1" false 0 "None"))
    (if _returnvalue_2
      (Transformation|SetWorldLocation (Variables|Default|GetEndLight) (+ (* (.Location (Collision|BreakHitResult _outhit)) 0.95) (* (.TraceStart (Collision|BreakHitResult _outhit)) 0.05)) false false)
      (else
        (Transformation|SetWorldLocation (Variables|Default|GetEndLight) (.TraceEnd (Collision|BreakHitResult _outhit)) false false)))))

(event Custom|PlaySound
  (params (Sound :type Sound%20Base%20Object%20Reference))
  ;[1 1 1] Sound Help
  (Utilities|IsValid Sound
    (:Is%20Valid
      (Audio|PlaySoundatLocation Sound (Transformation|GetWorldLocation (Variables|Default|GetPointer)) "0, 0, 0" 1.0 1.0 0.0 "/Game/Lightsaber/Sound/SaberSounds/SA_Basic.SA_Basic" 0 0))))

(event EventTick
  (params (DeltaSeconds :type Float%20%28single-precision%29))
  (bind _idlesound (Variables|Default|GetIdleSound))
  ;[1 1 1] Basic
  (CallFunction|ActivationTick)
  (CallFunction|LightPos)
  (CallFunction|DrawDecal)
  (CallFunction|ForceTick)
  (if (Variables|Default|GetisActive)
    (if (not (Audio|Components|Audio|IsPlaying (Variables|Default|GetIdleSound)))
      (Audio|Components|Audio|Play _idlesound 0.0)
      (Transformation|SetWorldLocation _idlesound (Transformation|GetWorldLocation (Variables|Default|GetPointer)) false false))
    (else
      (Audio|Components|Audio|Stop _idlesound))))

(event EventBeginPlay
  ;[1 1 1] Basic
  (CallFunction|Init))

(fn ConstructionScript
  (bind _width (Variables|Basic|GetWidth))
  (bind _saber (Variables|Default|GetSaber))
  (bind _width_2 (Variables|Basic|GetWidth))
  (bind _collisionmult (Variables|Basic|GetCollisionMult))
  (bind _length (Variables|Basic|GetLength))
  (bind _returnvalue (/ _width 1e+02))
  (bind _returnvalue_2 (* _width_2 _collisionmult))
  (Transformation|SetRelativeScale3D _saber (Math|Vector|MakeVector _returnvalue _returnvalue (/ _length 1e+02)))
  (Transformation|SetRelativeLocation _saber (Math|Vector|MakeVector 0.0 0.0 (/ _length 2.0)) false false)
  (Components|Box|SetBoxExtent (Variables|Default|GetCollision) (Math|Vector|MakeVector _returnvalue_2 _returnvalue_2 (/ (Variables|Basic|GetLength) 2.0)) true)
  (bind _returnvalue_3 (Rendering|Material|CreateDynamicMaterialInstance (Variables|Default|GetSaber) 0 "/Game/Lightsaber/Materials/Lightsaber/M_Saber_Base.M_Saber_Base" "None" :!class /Script/Engine.PrimitiveComponent))
  (Variables|Default|SetSaberMat _returnvalue_3)
  (CallFunction|SetColor (Variables|Basic|GetColor)))

(fn GetTargeting
  (bind _deflectdir (Variables|Default|GetDeflectDir))
  (return (Transformation|GetWorldLocation _deflectdir) (Math|Rotator|GetRotationXVector (Transformation|GetWorldRotation _deflectdir))))

(fn GetDeflect
  (bind _returnvalue (Actor|GetParentActor))
  (bind (_pos _dir) (CallFunction|GetTargeting))
  (bind _returnvalue_2 (Game|Player|GetPlayerPawn 0))
  (bind _autotargetingmode (Variables|AutoTargeting|GetautoTargetingMode))
  (bind _autotargetingmode_2 (Variables|AutoTargeting|GetautoTargetingMode))
  (bind _askylo_ren_saber (Utilities|Casting|CastToKyloRenSaber _returnvalue))
  (bind _asbp_motion_controller_pawn (Utilities|Casting|CastToBP_MotionControllerPawn _returnvalue_2))
  (bind (_pos_2 _dir_2) (Default|GetTargeting _asbp_motion_controller_pawn))
  (bind _hand (Variables|/Game/Lightsaber/Blueprints/HeroSabers/KyloRenSaber.KyloRenSaber_C|GetHand _askylo_ren_saber))
  (bind (_pos_3 _dir_3) (Default|GetTargeting _hand))
  (bind _returnvalue_3 (Utilities|Select :Index _autotargetingmode_2 :NewEnumerator0 _dir :NewEnumerator1 _dir_2 :NewEnumerator2 _dir_3))
  (bind _returnvalue_4 (Utilities|Select :Index _autotargetingmode :NewEnumerator0 _pos :NewEnumerator1 _pos_2 :NewEnumerator2 _pos_3))
  (bind (_x _y) (Math|Vector|BreakVector _returnvalue_3))
  (if (and (Variables|AutoTargeting|GetenableAutoTargeting) (Variables|Default|GetisActive))
    (bind _outhits (Collision|MultiSphereTraceByChannel _returnvalue_4 (+ _returnvalue_4 (* (Math|Vector|SelectVector (Math|Vector|MakeVector _x _y 0.0) _returnvalue_3 (Variables|AutoTargeting|GetautoTargetingHorizontal)) (+ (Variables|AutoTargeting|GetautoTargetigRadius) (Variables|AutoTargeting|GetautoTargetingLength)))) (Variables|AutoTargeting|GetautoTargetigRadius) "TraceTypeQuery1" false 0 (select (Variables|AutoTargeting|GetenableAutoTargetingDebug) "ForDuration" "None")))
    (for _array_element _outhits
      (if (Utilities|DoesObjectImplementInterface (.HitActor (Collision|BreakHitResult _array_element)) "/Game/Lightsaber/Blueprints/BI_Targetable.BI_Targetable_C")
        (Utilities|IsValid (LocalVariables|GetClosest)
          (:Is%20Valid
            (if (> (Math|Vector|VectorLength (- (Transformation|GetActorLocation (LocalVariables|GetClosest)) (.TraceEnd (Collision|BreakHitResult _array_element)))) (.Distance (Collision|BreakHitResult _array_element)))
              (LocalVariables|SetClosest (.HitActor (Collision|BreakHitResult _array_element)))))
          (:Is%20Not%20Valid
            (LocalVariables|SetClosest (.HitActor (Collision|BreakHitResult _array_element)))))))
    (Utilities|IsValid (LocalVariables|GetClosest)
      (:Is%20Valid
        (bind _location (Class|BITargetable|GetTarget(Message) (LocalVariables|GetClosest)))
        (return (Math|Vector|Normalize (- _location (Transformation|GetWorldLocation (Variables|Default|GetDeflectDir))))))
      (:Is%20Not%20Valid
        _)))
  (return (Math|Rotator|GetRotationXVector (Transformation|GetWorldRotation (Variables|Default|GetDeflectDir)))))