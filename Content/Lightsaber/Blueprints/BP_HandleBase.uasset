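; BP_HandleBase is a base lightsaber hilt that a hand can pick up, drop or optionally Force-grab.
; Pickup attaches the hilt to the hand's socket, while dropping detaches it, restores its physics setting and turns the blade off.
; A child-actor BP_SaberBase provides the blade, receiving on, off, toggle and color calls.
; Overlapping a BP_Crystal consumes it, recolors the blade and satisfies the optional crystal requirement for igniting.
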(event OnComponentBeginOverlap(CrystalCollision)
  (params (OverlappedComponent :type Primitive%20Component%20Object%20Reference) (OtherActor :type Actor%20Object%20Reference) (OtherComp :type Primitive%20Component%20Object%20Reference) (OtherBodyIndex :type Integer) (bFromSweep :type Boolean) (SweepResult :type Hit%20Result%20Structure%20%28by%20ref%29))
  (bind _asbp_crystal (Utilities|Casting|CastToBP_Crystal OtherActor))
  (CallFunction|UseCrystal _asbp_crystal)
  (Actor|DestroyActor _asbp_crystal))

(event Custom|TurnOn
  (if (or (Variables|Default|GethasCrystal) (not (Variables|Default|GetrequireCrystal)))
    (Default|Turnon (CallFunction|GetChildSaber (Variables|Default|GetSaber)))))

(event Custom|TurnOff
  (Default|TurnOff (CallFunction|GetChildSaber (Variables|Default|GetSaber))))

(event Custom|UseCrystal
  (params (Crystal :type BP%20Crystal%20Object%20Reference))
  (Variables|Default|SethasCrystal true)
  (Default|SetColor (CallFunction|GetChildSaber (Variables|Default|GetSaber)) (Variables|/Game/Lightsaber/Blueprints/MiscObjects/BP_Crystal.BP_Crystal_C|Getcolor Crystal)))

(event EventPickup
  (params (Hand :type BP%20Motion%20Controller%20Object%20Reference))
  (Variables|Default|SetHand Hand)
  (Transformation|AttachComponentToComponent (Variables|Default|GetHilt) (Variables|/Game/Lightsaber/Blueprints/BP_MotionController.BP_MotionController_C|GetHandMesh Hand) "Hilt" "SnapToTarget" "SnapToTarget" "KeepWorld" true)
  (Physics|SetSimulatePhysics (Variables|Default|GetHilt) false))

(event EventForceGrab
  (params (Hand :type BP%20Motion%20Controller%20Object%20Reference))
  (if (Variables|Default|GetenableForceGrab)
    (Utilities|BasicForceGrab Hand (Variables|Default|GetHilt))))

(event EventDrop
  (params (Hand :type BP%20Motion%20Controller%20Object%20Reference))
  (Transformation|DetachFromComponent (Variables|Default|GetHilt) "KeepWorld" "KeepWorld" "KeepWorld" true)
  (Physics|SetSimulatePhysics (Variables|Default|GetHilt) (Variables|Default|GetsimulatePhysics))
  (CallFunction|TurnOff))

(event EventBeginPlay
  (Physics|SetSimulatePhysics (Variables|Default|GetHilt) (Variables|Default|GetsimulatePhysics)))

(event EventFaceButton1Press
  (if (or (Variables|Default|GethasCrystal) (not (Variables|Default|GetrequireCrystal)))
    (Default|TurnToggle (CallFunction|GetChildSaber (Variables|Default|GetSaber)))))

(fn ConstructionScript
  (|CallParentFunction)
  (Default|SetColor (CallFunction|GetChildSaber (Variables|Default|GetSaber)) (Variables|Default|GetbaseColor)))

(fn GetChildSaber
  (params (ChildActor :type Child%20Actor%20Component%20Object%20Reference))
  (if true
    (bind _asbp_saber_base (Utilities|Casting|CastToBP_SaberBase (Variables|/Script/Engine.ChildActorComponent|GetChildActor ChildActor)))
    (return _asbp_saber_base)))

(fn GetParent
  (return (Transformation|GetAttachParent (Variables|Default|GetHilt))))