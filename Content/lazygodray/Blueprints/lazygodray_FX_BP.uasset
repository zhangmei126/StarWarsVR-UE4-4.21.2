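; Godray effect actor that builds a tinted light shaft card with optional dust particles and a spotlight, configured entirely in the construction script.
; It creates a dynamic material for the card, optionally an experimental converging variant, and pushes shaft, falloff, fade and smoke parameters into it.
; Length and diameter multipliers drive card scale, smoke tiling and panning, dust spawn volume and amount, and spotlight radius and cone angle.
; Event graph is empty, so toggling dust or spotlight at runtime needs extra work.
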(event EventBeginPlay)

(event Collision|EventActorBeginOverlap
  (params (OtherActor :type Actor%20Object%20Reference)))

(event EventTick
  (params (DeltaSeconds :type Float%20%28single-precision%29)))

(fn ConstructionScript
  (bind _diameter_multiplier (Variables|1.Scale|Getdiameter%20multiplier))
  (bind _godray_card_sm (Variables|Components|Getgodray_card_SM))
  (bind _smoke_texture_scale (Variables|4.RunningSmoke|Getsmoke%20texture%20scale))
  (bind _length_multiplier (Variables|1.Scale|Getlength%20multiplier))
  (bind _godray_card_sm_2 (Variables|Components|Getgodray_card_SM))
  (bind _size_multiplier (Variables|5.DustParticles|Getsize%20multiplier))
  (bind _velocity_multiplier (Variables|5.DustParticles|Getvelocity%20multiplier))
  (bind _spotlight (Variables|Components|Getspotlight))
  (bind _godray_card_sm_3 (Variables|Components|Getgodray_card_SM))
  (bind _godray_card_sm_4 (Variables|Components|Getgodray_card_SM))
  (bind _returnvalue (/ _length_multiplier 2.0))
  (bind _returnvalue_2 (* _velocity_multiplier 0.5))
  (Transformation|SetActorScale3D "1.000000,1.000000,1.000000")
  ;[1 1 1] lightray convergent experimental feature
  (if (Variables|3.VolumetricSettings|Getuse%20lightray%20convergent%20)
    (bind _returnvalue_3 (Rendering|Material|CreateDynamicMaterialInstance _godray_card_sm_2 0 (LocalVariables|Getconverging%20godray%20mtl) "None" :!class /Script/Engine.PrimitiveComponent))
    (LocalVariables|Setgodray%20mtl%20dynamic%20instance _returnvalue_3)
    (Rendering|Material|SetScalarParameterValueonMaterials (Variables|Components|Getgodray_card_SM) "lightray convergent" (Variables|3.VolumetricSettings|Getlightray%20convergent%20rate))
    (else
      (bind _returnvalue_4 (Rendering|Material|CreateDynamicMaterialInstance _godray_card_sm_2 0 (LocalVariables|Getgodray%20mtl) "None" :!class /Script/Engine.PrimitiveComponent))
      (LocalVariables|Setgodray%20mtl%20dynamic%20instance _returnvalue_4)))
  (Transformation|SetRelativeScale3D (Variables|Components|Getgodray_card_SM) (Math|Vector|MakeVector (Variables|1.Scale|Getlength%20multiplier) _diameter_multiplier _diameter_multiplier))
  ;[1 1 1] godray card material parameters
  (Rendering|Material|SetScalarParameterValueonMaterials _godray_card_sm_4 "overall intensity" (Variables|2.MainAttributes|Getoverall%20intensity))
  (Rendering|Material|SetVectorParameterValueonMaterials _godray_card_sm_4 "tint color" (Math|Conversions|ToVector(LinearColor) (Variables|2.MainAttributes|Gettint%20color)))
  (Rendering|Material|SetScalarParameterValueonMaterials _godray_card_sm_4 "overall contrast" (Variables|2.MainAttributes|Getoverall%20contrast))
  (Rendering|Material|SetScalarParameterValueonMaterials _godray_card_sm_4 "streak strength" (Variables|2.MainAttributes|Getlight%20shaft%20strength))
  (Rendering|Material|SetTextureParameterValue (LocalVariables|Getgodray%20mtl%20dynamic%20instance) "lightshaft texture" (Variables|2.MainAttributes|Getlight%20shaft%20texture))
  (Rendering|Material|SetScalarParameterValueonMaterials _godray_card_sm_4 "streaks amount multiplier" (Variables|2.MainAttributes|Getlight%20shaft%20amount))
  (Rendering|Material|SetScalarParameterValueonMaterials _godray_card_sm_4 "streaks length multiplier" (Variables|2.MainAttributes|Getlight%20shaft%20length))
  (Rendering|Material|SetScalarParameterValueonMaterials _godray_card_sm "depth fade" (Variables|3.VolumetricSettings|Getdepth%20fade%20distance))
  (Rendering|Material|SetScalarParameterValueonMaterials _godray_card_sm "fresnel exponent" (Variables|3.VolumetricSettings|Getfresnel%20exponent))
  (Rendering|Material|SetScalarParameterValueonMaterials _godray_card_sm "fading start distance" (Variables|3.VolumetricSettings|Getcamera%20fading%20start%20distance))
  (Rendering|Material|SetScalarParameterValueonMaterials _godray_card_sm "fading transition range" (Variables|3.VolumetricSettings|Getcamera%20fading%20transition%20range))
  (Rendering|Material|SetScalarParameterValueonMaterials _godray_card_sm "falloff strength" (Variables|3.VolumetricSettings|Getvertical%20falloff%20strength))
  (Rendering|Material|SetScalarParameterValueonMaterials _godray_card_sm "falloff midpoint" (Variables|3.VolumetricSettings|Getvertical%20falloff%20midpoint))
  (Rendering|Material|SetScalarParameterValueonMaterials _godray_card_sm "falloff exponent" (Variables|3.VolumetricSettings|Getvertical%20falloff%20exponent))
  (Rendering|Material|SetScalarParameterValueonMaterials _godray_card_sm "cylindrical falloff exponent" (Variables|3.VolumetricSettings|Getcylindrical%20masking%20exponent))
  (Rendering|Material|SetScalarParameterValueonMaterials _godray_card_sm_3 "detail intensity" (Variables|4.RunningSmoke|Getsmoke%20intensity))
  (Rendering|Material|SetTextureParameterValue (LocalVariables|Getgodray%20mtl%20dynamic%20instance) "masking texture" (Variables|4.RunningSmoke|Getsmoke%20texture))
  (Rendering|Material|SetScalarParameterValueonMaterials _godray_card_sm_3 "detail texture tilingX" (* _smoke_texture_scale (Variables|1.Scale|Getdiameter%20multiplier)))
  (Rendering|Material|SetScalarParameterValueonMaterials _godray_card_sm_3 "detail texture tilingY" (* _smoke_texture_scale (Variables|1.Scale|Getlength%20multiplier)))
  (Rendering|Material|SetScalarParameterValueonMaterials _godray_card_sm_3 "detail Xspeed" (/ (Variables|4.RunningSmoke|Getpanning%20speedX) (Variables|1.Scale|Getdiameter%20multiplier)))
  (Rendering|Material|SetScalarParameterValueonMaterials _godray_card_sm_3 "detail Yspeed" (/ (Variables|4.RunningSmoke|Getpanning%20speed%20Y) (Variables|1.Scale|Getlength%20multiplier)))
  ;[1 1 1] Particle System parameters
  (if (Variables|5.DustParticles|Getenable%20dust%20particle.%20cannot%20be%20toggled%20during%20runtime%20without%20further%20modification%20in%20blueprint.)
    (bind _returnvalue_5 (AddComponent|AddParticleSystemComponent false))
    (LocalVariables|Setgodray_dust _returnvalue_5)
    (bind _returnvalue_6 (Rendering|Material|CreateDynamicMaterialInstance (LocalVariables|Getgodray_dust) 0 (LocalVariables|Getdust%20mtl) "None" :!class /Script/Engine.PrimitiveComponent))
    (LocalVariables|Setdust%20mtl%20dynamic%20instance _returnvalue_6)
    (bind _output_get (LocalVariables|Setgodray_dust_parameters (Variables|/Script/Engine.ParticleSystemComponent|GetInstanceParameters (LocalVariables|Getgodray_dust))))
    (Utilities|Array|Add _output_get (Utilities|Struct|MakeParticleSysParam "size" "PSPT_VectorRand" 0.0 0.0 (Math|Conversions|ToVector(Float) _size_multiplier) (Math|Conversions|ToVector(Float) (* (/ (Variables|5.DustParticles|Getsize%20minimum%20percentage) 1e+02) _size_multiplier))))
    (Utilities|Array|Add _output_get (Utilities|Struct|MakeParticleSysParam "V" "PSPT_VectorRand" 0.0 0.0 (Math|Conversions|ToVector(Float) (+ _returnvalue_2 0.5)) (Math|Conversions|ToVector(Float) (- 0.5 _returnvalue_2))))
    (Variables|/Script/Engine.ParticleSystemComponent|SetInstanceParameters (LocalVariables|Getgodray_dust) _output_get)
    (Effects|Components|ParticleSystem|SetVectorParameter (LocalVariables|Getgodray_dust) "dust color" (Math|Conversions|ToVector(LinearColor) (Variables|5.DustParticles|Getparticle%20color)))
    (Transformation|SetRelativeLocation (LocalVariables|Getgodray_dust) (Math|Vector|MakeVector (* (+ _returnvalue (* (Variables|5.DustParticles|Getspawn%20location%20vertial%20offset) _returnvalue)) 1e+02) 0.0 0.0) false false)
    (Effects|Components|ParticleSystem|SetFloatParameter (LocalVariables|Getgodray_dust) "cylinderHeight" (* (* (Variables|1.Scale|Getlength%20multiplier) 1e+02) (Variables|5.DustParticles|Getspawn%20length%20multiplier)))
    (Effects|Components|ParticleSystem|SetFloatParameter (LocalVariables|Getgodray_dust) "cylinderRadius" (* (* (Variables|1.Scale|Getdiameter%20multiplier) 4e+01) (Variables|5.DustParticles|Getspawn%20radius%20multiplier)))
    (Effects|Components|ParticleSystem|SetFloatParameter (LocalVariables|Getgodray_dust) "spawn" (* (* (Variables|5.DustParticles|Getamount%20multiplier) (Variables|1.Scale|Getdiameter%20multiplier)) (Variables|1.Scale|Getlength%20multiplier)))
    (Effects|Components|ParticleSystem|SetFloatParameter (LocalVariables|Getgodray_dust) "revealing distance" (Variables|5.DustParticles|Getrevealing%20distance))
    (Effects|Components|ParticleSystem|SetFloatParameter (LocalVariables|Getgodray_dust) "revealing transition" (Variables|5.DustParticles|Getrevealing%20transition))
    (Effects|Components|ParticleSystem|SetFloatParameter (LocalVariables|Getgodray_dust) "culling distance" (Variables|5.DustParticles|Getculling%20distance))
    (Effects|Components|ParticleSystem|SetFloatParameter (LocalVariables|Getgodray_dust) "culling transition" (Variables|5.DustParticles|Getculling%20transition)))
  ;[1 1 1] spotlight parameters
  (Rendering|SetVisibility _spotlight (Variables|6.Spotlight|Getenable%20spotlight%20component;%20cannot%20be%20toggle%20during%20runtime%20without%20further%20modification%20in%20blueprint.) false)
  (Rendering|Lighting|SetAttenuationRadius _spotlight (+ (* (Variables|1.Scale|Getlength%20multiplier) 1e+02) (* (Variables|6.Spotlight|Getattenuation%20offset) (Variables|1.Scale|Getdiameter%20multiplier))))
  (Rendering|Lighting|SetOuterConeAngle _spotlight (+ (Class|KismetMathLibrary|DegAtan (/ (/ (Variables|1.Scale|Getdiameter%20multiplier) 2.0) (Variables|1.Scale|Getlength%20multiplier))) (Variables|6.Spotlight|Getouter%20cone%20angle%20offset)))
  (Rendering|Components|Light|SetLightColor _spotlight (Variables|2.MainAttributes|Gettint%20color) false)
  (Rendering|Components|Light|SetIntensity _spotlight (Variables|6.Spotlight|Getlight%20intensity))
  (Rendering|Lighting|SetInnerConeAngle _spotlight (Variables|6.Spotlight|Getinner%20cone%20angle%20))
  (Class|PointLightComponent|SetSourceRadius _spotlight (* (Variables|6.Spotlight|Getlight%20source%20radius) (Variables|1.Scale|Getdiameter%20multiplier))))